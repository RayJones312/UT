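; Character Blueprint that adds a multi-jump, allowing extra jumps in mid-air up to MaxJumps.
; Jump presses while falling increment the Jumps counter and, within the limit, launch the character upward at the movement component's JumpZVelocity.
; The launch overrides vertical velocity but keeps horizontal momentum, and landing resets the counter to one; grounded presses trigger nothing in this graph.
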(event EventOnLanded
  (params (Hit :type Hit%20Result%20Structure%20%28by%20ref%29))
  ;[1 1 1] Multi Jump
  (Variables|Default|SetJumps 1))

(event Input|ActionEvents|InputActionJump
  (bind _charactermovement (Variables|Character|GetCharacterMovement))
  ;[1 1 1] Multi Jump
  (:Pressed
    (if (AI|Components|NavMovement|IsFalling _charactermovement)
      (Variables|Default|SetJumps (+ (Variables|Default|GetJumps) 1))
      (if (<= (Variables|Default|GetJumps) (Variables|Default|GetMaxJumps))
        (Character|LaunchCharacter (Math|Vector|MakeVector 0.0 0.0 (Variables|/Script/Engine.CharacterMovementComponent|GetJumpZVelocity _charactermovement)) false true)))))

(fn ConstructionScript)